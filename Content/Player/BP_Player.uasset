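; Player character with a flipbook sprite, handling movement, look, jump, sprint and sword combat through Enhanced Input.
; Movement follows camera yaw and swaps walk and idle flipbooks; sprint changes max walk speed.
; Basic attack enables sword collision while held, damaging the first "Enemy"-tagged overlap using the Attack stat, then disabling collision.
; Incoming damage lowers Health in the Stats struct, and Tick destroys the actor once it reaches zero.
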(event `self.ReceiveBeginPlay`
  (bind _asbp_player_controller (cast `/Game/Player/BP_Player_Controller` (`GameplayStatics.GetPlayerController` 0)))
  (`EnhancedInputSubsystemInterface.AddMappingContext` (pcsubsystem `EnhancedInputLocalPlayerSubsystem` _asbp_player_controller) "/Game/Player/Inputs/IMC_Player_Actions.IMC_Player_Actions" 0 (struct)))

(event `EnhancedInput|/Game/Player/Inputs/IA_Jump`
  (params (ActionValue :type Boolean) (ElapsedSeconds :type "Float (double-precision)") (TriggeredSeconds :type "Float (double-precision)") (InputAction :type "InputAction Object Reference" :default "/Game/Player/Inputs/IA_Jump.IA_Jump"))
  (:`Started`
    (`self.Jump`)
    (`KismetSystemLibrary.PrintString` "Jumping!"))
  (:`Canceled`
    (`self.StopJumping`)))

(event `EnhancedInput|/Game/Player/Inputs/IA_Move`
  (params (ActionValue :type "Vector2D Structure") (ElapsedSeconds :type "Float (double-precision)") (TriggeredSeconds :type "Float (double-precision)") (InputAction :type "InputAction Object Reference" :default "/Game/Player/Inputs/IA_Move.IA_Move"))
  (bind (_x _y) (`KismetMathLibrary.BreakVector2D` ActionValue))
  (bind _returnvalue (`KismetMathLibrary.MakeRotator` 0.0 0.0 (.yaw (`SceneComponent.K2_GetComponentRotation` (`self.Player_Camera`)))))
  (:`Triggered`
    (`self.AddMovementInput` (`KismetMathLibrary.GetRightVector` _returnvalue) _x)
    (`self.AddMovementInput` (* (`KismetMathLibrary.GetForwardVector` _returnvalue) (-1.0 -1.0 -1.0)) _y)
    (`PaperFlipbookComponent.SetFlipbook` (`self.Sprite`) "/Game/Characters/Assets/Player_Walk_Up/Flipbook_Player_Walk_Up.Flipbook_Player_Walk_Up"))
  (:`Completed`
    (`PaperFlipbookComponent.SetFlipbook` (`self.Sprite`) "/Game/Characters/Assets/Player_idle/Flipbook_Player_Idle.Flipbook_Player_Idle")))

(event `EnhancedInput|/Game/Player/Inputs/IA_Basic_Attack`
  (params (ActionValue :type Boolean) (ElapsedSeconds :type "Float (double-precision)") (TriggeredSeconds :type "Float (double-precision)") (InputAction :type "InputAction Object Reference" :default "/Game/Player/Inputs/IA_Basic_Attack.IA_Basic_Attack"))
  (bind _sprite (`self.Sprite`))
  (bind _swordcollision (`self.SwordCollision`))
  (:`Started`
    (`KismetSystemLibrary.PrintString` "Attack! Hyah!")
    (`PaperFlipbookComponent.SetFlipbook` _sprite "/Game/Characters/Assets/Player_Attack/Flipbook_Character_Attack.Flipbook_Character_Attack")
    (`PrimitiveComponent.SetCollisionEnabled` _swordcollision "QueryOnly"))
  (:`Completed`
    (`PaperFlipbookComponent.SetFlipbook` _sprite "/Game/Characters/Assets/Player_idle/Flipbook_Player_Idle.Flipbook_Player_Idle")
    (`PrimitiveComponent.SetCollisionEnabled` _swordcollision "NoCollision")))

(event `self.SwordCollision.OnComponentBeginOverlap`
  (params (OverlappedComponent :type "PrimitiveComponent Object Reference") (OtherActor :type "Actor Object Reference") (OtherComp :type "PrimitiveComponent Object Reference") (OtherBodyIndex :type Integer) (bFromSweep :type Boolean) (SweepResult :type "HitResult Structure (by ref)"))
  (if (`self.ActorHasTag` OtherActor "Enemy")
    (`GameplayStatics.ApplyDamage` OtherActor (`.Attack_9_47D0D9494DE73D3F68CC6A912BA2CCB5` (break `/Game/Player/St_Player_Stats` (`self.Stats`))))
    (`PrimitiveComponent.SetCollisionEnabled` (`self.SwordCollision`) "NoCollision")))

(event `self.ReceiveTick`
  (params (DeltaSeconds :type "Float (single-precision)"))
  (if (<= (`.Health_4_D19E5AF34B4A93D92A71E1825CE21F4C` (break `/Game/Player/St_Player_Stats` (`self.Stats`))) 0.0)
    (`self.K2_DestroyActor`)))

(event `self.ReceiveAnyDamage`
  (params (Damage :type "Float (single-precision)") (DamageType :type "DamageType Object Reference") (InstigatedBy :type "Controller Object Reference") (DamageCauser :type "Actor Object Reference"))
  (bind (_health _speed _attack _mana) (break `/Game/Player/St_Player_Stats` (`self.Stats`)))
  (`KismetSystemLibrary.PrintString` (`KismetStringLibrary.Conv_DoubleToString` Damage))
  (set `self.Stats` (make `/Game/Player/St_Player_Stats` (- _health Damage) _speed _attack _mana))
  (`KismetSystemLibrary.PrintString` "WE NOW HAVE THIS MUCH HEALTH: ")
  (`KismetSystemLibrary.PrintString` (`KismetStringLibrary.Conv_DoubleToString` _health)))

(event `EnhancedInput|/Game/Player/Inputs/IA_Sprint`
  (params (ActionValue :type Boolean) (ElapsedSeconds :type "Float (double-precision)") (TriggeredSeconds :type "Float (double-precision)") (InputAction :type "InputAction Object Reference" :default "/Game/Player/Inputs/IA_Sprint.IA_Sprint"))
  (bind _charactermovement (`self.CharacterMovement`))
  (:`Triggered`
    (set `CharacterMovementComponent.MaxWalkSpeed` 1000.0 _charactermovement))
  (:`Completed`
    (set `CharacterMovementComponent.MaxWalkSpeed` 600.0 _charactermovement)))

(event `EnhancedInput|/Game/Player/Inputs/IA_Look_Horizontally`
  (params (ActionValue :type "Float (double-precision)") (ElapsedSeconds :type "Float (double-precision)") (TriggeredSeconds :type "Float (double-precision)") (InputAction :type "InputAction Object Reference" :default "/Game/Player/Inputs/IA_Look_Horizontally.IA_Look_Horizontally"))
  (:`Triggered`
    (`self.AddControllerYawInput` ActionValue)))

(event `EnhancedInput|/Game/Player/Inputs/IA_Look_Vertically`
  (params (ActionValue :type "Float (double-precision)") (ElapsedSeconds :type "Float (double-precision)") (TriggeredSeconds :type "Float (double-precision)") (InputAction :type "InputAction Object Reference" :default "/Game/Player/Inputs/IA_Look_Vertically.IA_Look_Vertically"))
  (:`Triggered`
    (`self.AddControllerPitchInput` (* ActionValue -1.0))))

(fn `TakeDamage`
  (`GameplayStatics.ApplyDamage` self)
  (`KismetSystemLibrary.PrintString` "OW BRUH????"))

(fn `UserConstructionScript`)