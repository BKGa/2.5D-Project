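; BP_Fireball is a short-lived fireball projectile that damages actors tagged Enemy.
; Each tick it passes its Fireball component to LookAtPlayerCamera, apparently to billboard the sprite toward the camera.
; A capsule overlap applies fixed damage to enemies and destroys the fireball, passes through actors tagged Player, and destroys it on anything else.
; A delay started at BeginPlay destroys it after a few seconds.
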(event `self.ReceiveTick`
  (params (DeltaSeconds :type "Float (single-precision)"))
  (`/Game/Enemies/BPL_Enemy_Functions.Look at Player Camera` (`self.Fireball`) self))

(event `self.ReceiveBeginPlay`
  (`KismetSystemLibrary.Delay` 3.0)
  (`self.K2_DestroyActor`))

(event `self.Capsule.OnComponentBeginOverlap`
  (params (OverlappedComponent :type "PrimitiveComponent Object Reference") (OtherActor :type "Actor Object Reference") (OtherComp :type "PrimitiveComponent Object Reference") (OtherBodyIndex :type Integer) (bFromSweep :type Boolean) (SweepResult :type "HitResult Structure (by ref)"))
  (if (`self.ActorHasTag` OtherActor "Enemy")
    (`GameplayStatics.ApplyDamage` OtherActor 10.0)
    (`self.K2_DestroyActor` :!label _label)
    (elif (not (`self.ActorHasTag` OtherActor "Player"))
      (goto _label))))

(fn `UserConstructionScript`)