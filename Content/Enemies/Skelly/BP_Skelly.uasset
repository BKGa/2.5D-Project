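; BP_Skelly is a skeleton enemy with a sprite that yaws to face the camera and a melee hitbox.
; Tick moves the hitbox to whichever X side the player is on and destroys the actor once health runs out.
; Seeing BP_Player through PawnSensing sets a blackboard flag for the AI.
; Hitbox overlaps deal Attack damage to Player-tagged actors, while incoming damage reduces Stats.Health and prints a debug string.
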(event `self.ReceiveTick`
  (params (DeltaSeconds :type "Float (single-precision)"))
  (bind _returnvalue_x (`KismetMathLibrary.BreakVector` (`self.K2_GetActorLocation`)))
  (bind _hitbox (`self.Hitbox`))
  (bind _returnvalue_x_2 (`KismetMathLibrary.BreakVector` (`self.K2_GetActorLocation` (`GameplayStatics.GetPlayerCharacter` 0))))
  (bind (_returnvalue_roll _returnvalue_pitch _returnvalue_yaw) (`KismetMathLibrary.BreakRotator` (`KismetMathLibrary.FindLookAtRotation` (`self.K2_GetActorLocation`) (`PlayerCameraManager.GetCameraLocation` (`GameplayStatics.GetPlayerCameraManager` 0)))))
  (`SceneComponent.K2_SetWorldRotation` (`self.Sprite`) (`KismetMathLibrary.MakeRotator` 0.0 0.0 (+ _returnvalue_yaw 90.0)) false false)
  (if (< _returnvalue_x _returnvalue_x_2)
    (`SceneComponent.K2_SetRelativeLocation` _hitbox (110.0 0.0 20.0) false false)
    (else
      (`SceneComponent.K2_SetRelativeLocation` _hitbox (-110.0 0.0 20.0) false false)))
  (if (<= (`.Health_2_9F107D78469D05BE0FE43CA9D3C1A939` (break `/Game/Enemies/St_Enemy_Stats` (`self.Stats`))) 0.0)
    (`self.K2_DestroyActor`)))

(event `self.ReceiveAnyDamage`
  (params (Damage :type "Float (single-precision)") (DamageType :type "DamageType Object Reference") (InstigatedBy :type "Controller Object Reference") (DamageCauser :type "Actor Object Reference"))
  (bind (_health _attack _speed _mana) (break `/Game/Enemies/St_Enemy_Stats` (`self.Stats`)))
  (set `self.Stats` (make `/Game/Enemies/St_Enemy_Stats` (- _health Damage) _attack _speed _mana))
  (`KismetSystemLibrary.PrintString` "DAMN BRUH THAT HURT"))

(event `self.PawnSensing.OnSeePawn`
  (params (Pawn :type "Pawn Object Reference"))
  (cast `/Game/Player/BP_Player` Pawn)
  (`BlackboardComponent.SetValueAsBool` (`AIBlueprintHelperLibrary.GetBlackboard` (`AIBlueprintHelperLibrary.GetAIController` self)) "hasSeenPlayer?" true))

(event `self.Hitbox.OnComponentBeginOverlap`
  (params (OverlappedComponent :type "PrimitiveComponent Object Reference") (OtherActor :type "Actor Object Reference") (OtherComp :type "PrimitiveComponent Object Reference") (OtherBodyIndex :type Integer) (bFromSweep :type Boolean) (SweepResult :type "HitResult Structure (by ref)"))
  (if (`self.ActorHasTag` OtherActor "Player")
    (`GameplayStatics.ApplyDamage` OtherActor (`.Attack_4_E61E00B944C77F832E82738C1033EF71` (break `/Game/Enemies/St_Enemy_Stats` (`self.Stats`))))))

(fn `Take Damage`
  (`GameplayStatics.ApplyDamage` self))

(fn `UserConstructionScript`)