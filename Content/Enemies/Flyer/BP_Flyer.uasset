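; BP_Flyer is a sprite-based flying enemy that detects allies and flags them to its AI, apparently for buffing.
; BeginPlay enables the buff Blackboard key, and Tick turns the sprite toward the player camera and checks for death.
; Pawn sensing stores Enemy-tagged pawns, sets the ally-seen key and tints the sprite until that ally is destroyed.
; Incoming damage reduces Health in its stats struct and prints a debug message.
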(event `self.ReceiveBeginPlay`
  (`BlackboardComponent.SetValueAsBool` (`AIBlueprintHelperLibrary.GetBlackboard` (`AIBlueprintHelperLibrary.GetAIController` self)) "CanBuff?" true))

(event `self.ReceiveTick`
  (params (DeltaSeconds :type "Float (single-precision)"))
  (`/Game/Enemies/BPL_Enemy_Functions.Look at Player Camera` (`self.Sprite`) self)
  (`/Game/Enemies/BPL_Enemy_Functions.Check If Dead` (`self.Flyer Stats`) self))

(event `self.PawnSensing.OnSeePawn`
  (params (Pawn :type "Pawn Object Reference"))
  (if (`self.ActorHasTag` Pawn "Enemy")
    (set `self.Seen Ally Actor` Pawn)
    (`BlackboardComponent.SetValueAsBool` (`AIBlueprintHelperLibrary.GetBlackboard` (`AIBlueprintHelperLibrary.GetAIController` self)) "hasSeenAlly?" true)
    (`PaperFlipbookComponent.SetSpriteColor` (`self.Sprite`) (struct :`R` 0.432712 :`G` 0.355765 :`B` 1.0 :`A` 1.0))
    (add `self.OnDestroyed` Pawn (delegate `OnDestroyed_Event`))))

(event `OnDestroyed_Event` :!signature `self.OnDestroyed`
  (params (DestroyedActor :type "Actor Object Reference"))
  (`BlackboardComponent.SetValueAsBool` (`AIBlueprintHelperLibrary.GetBlackboard` (`AIBlueprintHelperLibrary.GetAIController` self)) "hasSeenAlly?" false)
  (`PaperFlipbookComponent.SetSpriteColor` (`self.Sprite`) (struct :`R` 1.0 :`G` 1.0 :`B` 1.0 :`A` 1.0)))

(event `self.ReceiveAnyDamage`
  (params (Damage :type "Float (single-precision)") (DamageType :type "DamageType Object Reference") (InstigatedBy :type "Controller Object Reference") (DamageCauser :type "Actor Object Reference"))
  (bind (_health _attack _speed _mana) (break `/Game/Enemies/St_Enemy_Stats` (`self.Flyer Stats`)))
  (set `self.Flyer Stats` (make `/Game/Enemies/St_Enemy_Stats` (- _health Damage) _attack _speed _mana))
  (`KismetSystemLibrary.PrintString` "YOU HIT THE FLYER?????" true true (struct :`R` 0.260921 :`G` 0.154644 :`B` 1.0 :`A` 1.0)))

(fn `UserConstructionScript`)